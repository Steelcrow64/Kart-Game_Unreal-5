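; Physics-driven player kart that races along a BP_TrackSpline, with Enhanced Input for throttle and steering.
; Each tick, four wheel traces apply spring-like suspension and drive forces to the Box body, with airborne downforce and throttle-shifted center of mass.
; Steering applies throttle-scaled torque, and timed boosts scale drive force.
; The spline provides direction checks, lap-based course progress and a respawn point, with a delayed timer started when the kart topples.
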(event Input|EnhancedActionEvents|EnhancedInputActionIA_Acceleration
  (params (ActionValue :type Float%20%28double-precision%29) (ElapsedSeconds :type Float%20%28double-precision%29) (TriggeredSeconds :type Float%20%28double-precision%29) (InputAction :type Input%20Action%20Object%20Reference :default "/Game/Inputs/IA_Acceleration.IA_Acceleration"))
  (Variables|Default|SetAccelerationInput (Math|Interpolation|FInterpTo (Variables|Default|GetAccelerationInput) (Math|Float|SelectFloat ActionValue (Variables|Default|GetAccelerationInput) (CallFunction|IsonGround)) (Utilities|Time|GetWorldDeltaSeconds) 0.5)))

(event Input|EnhancedActionEvents|EnhancedInputActionIA_Steering
  (params (ActionValue :type Float%20%28double-precision%29) (ElapsedSeconds :type Float%20%28double-precision%29) (TriggeredSeconds :type Float%20%28double-precision%29) (InputAction :type Input%20Action%20Object%20Reference :default "/Game/Inputs/IA_Steering.IA_Steering"))
  (Class|PrimitiveComponent|AddTorqueinRadians (Variables|Default|GetBox) (Math|Vector|MakeVector 0.0 0.0 (* ActionValue (Variables|Default|GetSteeringTorque) (* (Variables|Default|GetAccelerationInput) (Variables|Default|GetSteeringMultiplier)))) "None" false)
  (Transformation|SetRelativeRotation (Variables|Default|GetFR_Wheel) (Math|Rotator|MakeRotator 0.0 0.0 (Math|Interpolation|FInterpTo (.yaw (Variables|/Script/Engine.SceneComponent|GetRelativeRotation (Variables|Default|GetFR_Wheel))) ActionValue (Utilities|Time|GetWorldDeltaSeconds) 3.0)) false false))

(event EventTick
  (params (DeltaSeconds :type Float%20%28single-precision%29))
  (CallFunction|SuspensionCast (Variables|Default|GetFL_Wheel))
  (CallFunction|SuspensionCast (Variables|Default|GetFR_Wheel))
  (CallFunction|SuspensionCast (Variables|Default|GetBR_Wheel))
  (CallFunction|SuspensionCast (Variables|Default|GetBL_Wheel))
  (CallFunction|CalculateAcceleration)
  (CallFunction|IsToppled))

(event EventBeginPlay
  (Input|AddMappingContext (PlayerController|LocalPlayerSubsystems|GetEnhancedInputLocalPlayerSubsystem (Game|GetPlayerController 0)) "/Game/Inputs/IMC_Vehicle.IMC_Vehicle" 0 "(bIgnoreAllPressedKeysUntilRelease=True,bForceImmediately=False,bNotifyUserSettings=False)")
  (bind _returnvalue (Actor|GetActorOfClass "/Game/Blueprints/BP_TrackSpline.BP_TrackSpline_C"))
  (Variables|Default|SetTrack _returnvalue)
  (bind _returnvalue_2 (UserInterface|CreateWidget "/Game/UI/W_HUD.W_HUD_C"))
  (UserInterface|Viewport|AddtoViewport _returnvalue_2 0))

(fn ConstructionScript)

(fn SuspensionCast
  (params (WheelComp :type Scene%20Component%20Object%20Reference))
  (bind _returnvalue (Transformation|GetWorldLocation WheelComp))
  (bind _returnvalue_2 (Components|GetChildComponent WheelComp 0))
  (bind _outhit (Collision|LineTraceByChannel _returnvalue (+ _returnvalue (* (Math|Vector|GetUpVector WheelComp) -6e+01)) "TraceTypeQuery1" false 0 "ForOneFrame"))
  (if (.bBlockingHit (Collision|BreakHitResult _outhit))
    (Class|PrimitiveComponent|AddForceatLocation (Variables|Default|GetBox) (* (- 1.0 (Math|Float|NormalizetoRange (.Distance (Collision|BreakHitResult _outhit)) 0.0 6e+01)) (Math|Vector|GetUnitDirection(Vector) (.TraceEnd (Collision|BreakHitResult _outhit)) (.TraceStart (Collision|BreakHitResult _outhit))) 9e+04) (Transformation|GetWorldLocation WheelComp) "None")
    (CallFunction|AccelerateKart WheelComp)
    (Transformation|SetRelativeLocation _returnvalue_2 (Math|Vector|MakeVector 0.0 0.0 (Math|Interpolation|FInterpTo (.z (Variables|/Script/Engine.SceneComponent|GetRelativeLocation _returnvalue_2)) (+ (* (.Distance (Collision|BreakHitResult _outhit)) -1.0) 25.0) (Utilities|Time|GetWorldDeltaSeconds) 3.0)) false false)
    (else
      (CallFunction|AccelerateKart WheelComp))))

(fn CalculateAcceleration
  (bind _output_get (Variables|Default|SetAcceleration (* (Math|Float|Lerp 0.0 (Variables|Default|GetMaxAcceleration) (Variables|Default|GetAccelerationInput)) (Variables|Default|GetAccelerationInput))))
  (Variables|Default|SetAccelerationInput (Math|Interpolation|FInterpTo (Variables|Default|GetAccelerationInput) 0.0 (Utilities|Time|GetWorldDeltaSeconds) 0.3))
  (Transformation|AddLocalRotation (Variables|Default|GetWheel_BL) (Math|Rotator|MakeRotator 0.0 0.0 (/ _output_get -1e+03)) false false))

(fn AccelerateKart
  (params (WheelComp :type Scene%20Component%20Object%20Reference))
  (bind _box (Variables|Default|GetBox))
  (Class|PrimitiveComponent|AddForceatLocation (Variables|Default|GetBox) (+ (* (Math|Vector|GetForwardVector _box) 2e+03 (Variables|Default|GetAccelerationInput) (Physics|GetMass _box) (Variables|Default|GetSpeedModifier)) (Math|Vector|SelectVector "0, 0, 0" (Math|Vector|MakeVector 0.0 0.0 (Variables|Default|GetDown%20Force)) (CallFunction|IsonGround))) (Transformation|GetWorldLocation WheelComp) "None")
  (Class|PrimitiveComponent|SetCenterOfMass (Variables|Default|GetBox) (* "50.000000,0.000000,0.000000" (Variables|Default|GetAccelerationInput)) "None"))

(fn IsonGround
  (bind _returnvalue (Transformation|GetActorLocation))
  (bind _returnvalue_2 (Collision|LineTraceByChannel _returnvalue (- _returnvalue "0.000000,0.000000,35.000000") "TraceTypeQuery1" false 0 "None"))
  (return _returnvalue_2))

(fn GetTrackProgress
  (return (> (Math|Vector|DotProduct (Spline|FindDirectionClosesttoWorldLocation (Variables|/Game/Blueprints/BP_TrackSpline.BP_TrackSpline_C|GetSpline (Variables|Default|GetTrack)) (Transformation|GetActorLocation) "World") (Math|Vector|Normalize (Transformation|GetVelocity))) 0.0)))

(fn BoostKart
  (params (SpeedModifier :type Float%20%28single-precision%29) (Time :type Float%20%28single-precision%29))
  (Variables|Default|SetSpeedModifier SpeedModifier)
  (Utilities|Time|SetTimerbyFunctionName 0 "ResetSpeed" Time))

(fn ResetSpeed
  (Variables|Default|SetSpeedModifier 1.0))

(fn GetCourseProgress
  (bind _track (Variables|Default|GetTrack))
  (bind _spline (Variables|/Game/Blueprints/BP_TrackSpline.BP_TrackSpline_C|GetSpline _track))
  (return (+ (/ (Class|SplineComponent|GetDistanceAlongSplineatLocation _spline (Spline|FindLocationClosesttoWorldLocation (Variables|/Game/Blueprints/BP_TrackSpline.BP_TrackSpline_C|GetSpline _track) (Transformation|GetActorLocation) "Local") "Local") (Spline|GetSplineLength _spline)) (Variables|Default|GetLaps))))

(fn IsToppled
  (if (and (< (Math|Vector|DotProduct (Transformation|GetActorUpVector) "0.000000,0.000000,1.000000") 0.8) (not (Utilities|Time|IsValidTimerHandle (Variables|Default|GetResetTimer))))
    (bind _returnvalue (Utilities|Time|SetTimerbyEvent (EventDispatchers|CreateEvent :!event ResetPosition) 3.0))
    (Variables|Default|SetResetTimer _returnvalue)))

(fn ResetPosition
  (bind _returnvalue (Transformation|GetActorLocation))
  (bind _track (Variables|Default|GetTrack))
  (bind _spline (Variables|/Game/Blueprints/BP_TrackSpline.BP_TrackSpline_C|GetSpline _track))
  (Utilities|Time|ClearandInvalidateTimerbyHandle (Variables|Default|GetResetTimer))
  (Transformation|SetActorLocationAndRotation (Spline|FindLocationClosesttoWorldLocation _spline _returnvalue "World") (Math|Conversions|RotationFromXVector (Spline|FindDirectionClosesttoWorldLocation _spline _returnvalue "World")))
  (Variables|Default|SetAccelerationInput 0.0))