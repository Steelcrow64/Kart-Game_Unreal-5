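; BP_FinishLine is a finish line actor that keeps a lap count for karts crossing it.
; On a BP_Kart overlap, it increments its LapCount and resets a DoOnce if GetTrackProgress returns true.
; Otherwise the DoOnce lets LapCount drop only once until the next reset.
; The count lives on the line rather than per kart, and Tick prints it every frame.
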(event Collision|EventActorBeginOverlap
  (params (OtherActor :type Actor%20Object%20Reference))
  (bind _asbp_kart (Utilities|Casting|CastToBP_Kart OtherActor))
  (if (Default|GetTrackProgress _asbp_kart)
    (Math|Integer|IncrementInt (Variables|Default|GetLapCount)
      (:%20%20
        (goto _label Reset)))
    (else
      (Utilities|FlowControl|DoOnce false :!label _label
        (:Completed
          (Math|Integer|DecrementInt (Variables|Default|GetLapCount)))))))

(event EventTick
  (params (DeltaSeconds :type Float%20%28single-precision%29))
  (Development|PrintString (Utilities|String|ToString(Integer) (Variables|Default|GetLapCount)) true true "(R=0.000000,G=0.660000,B=1.000000,A=1.000000)" 0.0))

(fn ConstructionScript)